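; Player pawn Blueprint that toggles its spring arm between first-person and third-person placements with the V key.
; BeginPlay caches the spring arm's initial relative transform as the third-person view, storing rotation as a forward (X) vector.
; Each press checks and flips SwitchToFirstPerson, applying either the first-person variables or the cached values.
; No movement logic is present; MovementSpeed is unused.
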(event `self.ReceiveBeginPlay`
  (set `self.ThirdPersonLocation` (`SceneComponent.RelativeLocation` (`self.SpringArm`)))
  (set `self.ThirdPersonRotation` (`KismetMathLibrary.Conv_RotatorToVector` (`SceneComponent.RelativeRotation` (`self.SpringArm`)))))

(event `Key|W`
  (params (Key :type "Key Structure")))

(event `Key|V`
  (params (Key :type "Key Structure"))
  (:`Pressed`
    (if (`self.SwitchToFirstPerson`)
      (`SceneComponent.K2_SetRelativeLocationAndRotation` (`self.SpringArm`) (`self.FirstPersonLocation`) (`KismetMathLibrary.Conv_VectorToRotator` (`self.FirstPersonRotation`)) false false)
      (set `self.SwitchToFirstPerson` false)
      (else
        (`SceneComponent.K2_SetRelativeLocationAndRotation` (`self.SpringArm`) (`self.ThirdPersonLocation`) (`KismetMathLibrary.Conv_VectorToRotator` (`self.ThirdPersonRotation`)) false false)
        (set `self.SwitchToFirstPerson` true)))))

(fn `UserConstructionScript`)